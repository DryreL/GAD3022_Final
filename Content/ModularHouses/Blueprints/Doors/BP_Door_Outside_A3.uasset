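; Hinged exterior door Blueprint from the ModularHouses content that the player opens and closes with E while inside its trigger.
; Trigger overlap toggles input for player controller 0 and prints a "Press E" prompt on entry, without checking the overlapping actor.
; A timeline plays or reverses to drive door yaw, with IsClosed staying true until the angle reaches 90 degrees.
; The Construction Script assigns the door's two materials from variables.
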(event OnComponentEndOverlap(Trigger)
  (params (OverlappedComponent :type Primitive%20Component%20Object%20Reference) (OtherActor :type Actor%20Object%20Reference) (OtherComp :type Primitive%20Component%20Object%20Reference) (OtherBodyIndex :type Integer))
  (Input|DisableInput (Game|GetPlayerController 0)))

(event OnComponentBeginOverlap(Trigger)
  (params (OverlappedComponent :type Primitive%20Component%20Object%20Reference) (OtherActor :type Actor%20Object%20Reference) (OtherComp :type Primitive%20Component%20Object%20Reference) (OtherBodyIndex :type Integer) (bFromSweep :type Boolean) (SweepResult :type Hit%20Result%20Structure%20%28by%20ref%29))
  (Input|EnableInput (Game|GetPlayerController 0))
  (Development|PrintText "Press E" true false "(R=1.000000,G=1.000000,B=1.000000,A=1.000000)" 1.0))

(event Input|KeyboardEvents|E
  (params (Key :type Key%20Structure :default "None"))
  (:Pressed
    (if (Variables|Default|GetIsClosed)
      (bind _newtrack_1 (Timeline|Timeline_0 Play)
        (:Update
          (Transformation|SetRelativeRotation (Variables|Default|GetDoor) (Math|Rotator|MakeRotator 0.0 0.0 _newtrack_1) false false)
          (if (>= _newtrack_1 9e+01)
            (Variables|Default|SetIsClosed false)
            (else
              (Variables|Default|SetIsClosed true)))))
      (else
        (Timeline|Timeline_0 Reverse)))))

(fn ConstructionScript
  (bind _door (Variables|Default|GetDoor))
  (Rendering|Material|SetMaterial _door 1 (Variables|Default|GetElement%200))
  (Rendering|Material|SetMaterial _door 0 (Variables|Default|GetElement%202)))