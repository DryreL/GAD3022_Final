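; BP_Ground_01 is a resizable ground piece from the ModularHouses road blueprints, sized by its Width and Lenght variables.
; The construction script converts Width and Lenght into the X and Y scale of its static mesh, leaving Z unchanged.
; It then creates a dynamic instance of Material and derives Tile_U and Tile_V linearly from those dimensions, so texture tiling follows the size.
; It has no active runtime logic.
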(event EventBeginPlay)

(event Collision|EventActorBeginOverlap
  (params (OtherActor :type Actor%20Object%20Reference)))

(event EventTick
  (params (DeltaSeconds :type Float%20%28single-precision%29)))

(fn ConstructionScript
  (bind _staticmeshcomponent (Variables|Debug|GetStaticMeshComponent))
  (bind _staticmeshcomponent_2 (Variables|Debug|GetStaticMeshComponent))
  (bind _relativescale3d (Variables|/Script/Engine.SceneComponent|GetRelativeScale3D _staticmeshcomponent_2))
  (bind (_x _y _z) (Math|Vector|BreakVector _relativescale3d))
  (Transformation|SetRelativeScale3D _staticmeshcomponent (Math|Vector|MakeVector _x (* (Variables|Default|GetLenght) 0.010755) _z))
  (Transformation|SetRelativeScale3D _staticmeshcomponent (Math|Vector|MakeVector (* (Variables|Default|GetWidth) 0.010755) _y _z))
  (bind _returnvalue (Rendering|Material|CreateDynamicMaterialInstance (Variables|Debug|GetStaticMeshComponent) 0 (Variables|Default|GetMaterial) :!class /Script/Engine.PrimitiveComponent))
  (Rendering|Material|SetScalarParameterValue _returnvalue "Tile_U" (+ (* (- (Math|Conversions|ToFloat(Integer) (Variables|Default|GetWidth)) 1.1e+02) 0.00625) 0.7) :!class /Script/Engine.MaterialInstanceDynamic)
  (Rendering|Material|SetScalarParameterValue _returnvalue "Tile_V" (+ (* (- (Math|Conversions|ToFloat(Integer) (Variables|Default|GetLenght)) 1.1e+02) 0.00625) 0.7) :!class /Script/Engine.MaterialInstanceDynamic))