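; BP_SideWalk_A1 is a modular sidewalk piece whose length along X follows its Width variable.
; The construction script stretches the Side spline mesh from StartTransform to an end point using Width and End's Y and Z.
; Tangents come from each transform's forward vector and scale, multiplied by the distance between the two transforms.
; A dynamic material on slot 1 adjusts Tile_V with Width to scale texture tiling.
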(fn ConstructionScript
  (bind _end (Variables|Default|GetEnd))
  (bind _end_transform (Variables|Default|GetEnd%20transform))
  (bind _start_transform (Variables|Default|GetStart%20transform))
  (bind (_location _rotation _scale) (Math|Transform|BreakTransform _start_transform))
  (bind (_x _y _z) (Math|Vector|BreakVector _end))
  (bind (_location_2 _rotation_2 _scale_2) (Math|Transform|BreakTransform _end_transform))
  (bind _returnvalue (- _location _location_2))
  (bind _returnvalue_2 (Math|Vector|VectorLength _returnvalue))
  (SplineMesh|SetStartandEnd (Variables|Default|GetSide) _location (* (* (Math|Vector|GetForwardVector _rotation) _scale) _returnvalue_2) (Math|Vector|MakeVector (Variables|Default|GetWidth) _y _z) (* (* (Math|Vector|GetForwardVector _rotation_2) _scale_2) _returnvalue_2) true :!class /Script/Engine.SplineMeshComponent)
  (bind _returnvalue_3 (Rendering|Material|CreateDynamicMaterialInstance (Variables|Default|GetSide) 1 (Variables|Default|GetElement%200) :!class /Script/Engine.PrimitiveComponent))
  (Rendering|Material|SetScalarParameterValue _returnvalue_3 "Tile_V" (+ (* (- (Variables|Default|GetWidth) 1.2e+02) 0.00625) 0.7) :!class /Script/Engine.MaterialInstanceDynamic))