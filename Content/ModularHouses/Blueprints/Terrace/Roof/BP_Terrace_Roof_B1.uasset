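; Construction-script Blueprint for a modular house terrace roof piece with adjustable width and optional rails.
; It bends the Side spline mesh from StartTransform to a Width-driven end, with tangents from each transform's rotation and scale, multiplied by their distance.
; Static meshes are added at both ends, each hideable along with its shadow.
; Materials are assigned to all parts, and a dynamic instance scales Side's U tiling with Width.
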(fn ConstructionScript
  (bind _width (Variables|Default|GetWidth))
  (bind _end (Variables|Default|GetEnd))
  (bind _end_transform (Variables|Default|GetEnd%20transform))
  (bind _start_transform (Variables|Default|GetStart%20transform))
  (bind (_location _rotation _scale) (Math|Transform|BreakTransform _start_transform))
  (bind (_x _y _z) (Math|Vector|BreakVector _end))
  (bind (_location_2 _rotation_2 _scale_2) (Math|Transform|BreakTransform _end_transform))
  (bind _returnvalue (Math|Vector|MakeVector _width _y _z))
  (bind _returnvalue_2 (- _location _location_2))
  (bind _returnvalue_3 (Math|Vector|VectorLength _returnvalue_2))
  (SplineMesh|SetStartandEnd (Variables|Default|GetSide) _location (* (* (Math|Vector|GetForwardVector _rotation) _scale) _returnvalue_3) _returnvalue (* (* (Math|Vector|GetForwardVector _rotation_2) _scale_2) _returnvalue_3) true :!class /Script/Engine.SplineMeshComponent)
  (bind _returnvalue_4 (AddComponent|AddStaticMeshComponent false _start_transform))
  (bind _returnvalue_5 (AddComponent|AddStaticMeshComponent false (Math|Conversions|ToTransform(Vector) _returnvalue)))
  (Rendering|Material|SetMaterial _returnvalue_5 0 (Variables|Default|GetMaterial_1))
  (Rendering|Material|SetMaterial _returnvalue_5 2 (Variables|Default|GetMaterial_2))
  (bind _returnvalue_6 (Rendering|Material|CreateDynamicMaterialInstance (Variables|Default|GetSide) 0 (Variables|Default|GetMaterial_1) :!class /Script/Engine.PrimitiveComponent))
  (Rendering|Material|SetScalarParameterValue _returnvalue_6 "Tile_U" (+ (* (- (Variables|Default|GetWidth) 1.2e+02) 0.01625) 1.0) :!class /Script/Engine.MaterialInstanceDynamic)
  (if (Variables|Default|GetHide%20Rail%202)
    (Rendering|SetVisibility _returnvalue_5 false false)
    (Rendering|SetCastShadow _returnvalue_5 false))
  (if (Variables|Default|GetHide%20Rail_1)
    (Rendering|SetVisibility _returnvalue_4 false false)
    (Rendering|SetCastShadow _returnvalue_4 false)))