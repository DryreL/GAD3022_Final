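; BP_Terrace_Base_A is a modular house terrace base that builds itself in the construction script from Width and Lenght.
; Side and Top spline meshes stretch from StartTransform to a Width-based end point, with tangents scaled by the start-to-end transform distance.
; Static meshes are added at both ends, one per end scaled in Y by Lenght, as is Top.
; Dynamic material instances adjust Tile_U and Tile_V to match the dimensions.
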(fn ConstructionScript
  (bind _top (Variables|Default|GetTop))
  (bind _element_0 (Variables|Default|GetElement%200))
  (bind _lenght (Variables|Default|GetLenght))
  (bind _width (Variables|Default|GetWidth))
  (bind _element_0_2 (Variables|Default|GetElement%200))
  (bind _end (Variables|Default|GetEnd))
  (bind _width_2 (Variables|Default|GetWidth))
  (bind _end_transform (Variables|Default|GetEnd%20transform))
  (bind _start_transform (Variables|Default|GetStart%20transform))
  (bind (_location _rotation _scale) (Math|Transform|BreakTransform _start_transform))
  (bind (_x _y _z) (Math|Vector|BreakVector _end))
  (bind _returnvalue (- _width_2 1.2e+02))
  (bind (_location_2 _rotation_2 _scale_2) (Math|Transform|BreakTransform _end_transform))
  (bind _returnvalue_2 (/ _lenght 0.5))
  (bind _relativescale3d (Variables|/Script/Engine.SceneComponent|GetRelativeScale3D _top))
  (bind (_x_2 _y_2 _z_2) (Math|Vector|BreakVector _relativescale3d))
  (bind _returnvalue_3 (Math|Vector|MakeVector _width _y _z))
  (bind _returnvalue_4 (Math|Conversions|ToTransform(Vector) _location))
  (bind _returnvalue_5 (Math|Vector|GetForwardVector _rotation))
  (bind _returnvalue_6 (Math|Vector|GetForwardVector _rotation_2))
  (bind _returnvalue_7 (- _location _location_2))
  (bind _returnvalue_8 (* _returnvalue 0.00625))
  (bind _returnvalue_9 (Math|Conversions|ToTransform(Vector) _returnvalue_3))
  (bind _returnvalue_10 (Math|Vector|VectorLength _returnvalue_7))
  (bind _returnvalue_11 (* _returnvalue_5 _scale))
  (bind _returnvalue_12 (* _returnvalue_6 _scale_2))
  (bind _returnvalue_13 (+ _returnvalue_8 1.0))
  (bind _returnvalue_14 (* _returnvalue_11 _returnvalue_10))
  (bind _returnvalue_15 (* _returnvalue_12 _returnvalue_10))
  (SplineMesh|SetStartandEnd (Variables|Default|GetSide) _location _returnvalue_14 _returnvalue_3 _returnvalue_15 true :!class /Script/Engine.SplineMeshComponent)
  (SplineMesh|SetStartandEnd (Variables|Default|GetTop) _location _returnvalue_14 _returnvalue_3 _returnvalue_15 true :!class /Script/Engine.SplineMeshComponent)
  (Transformation|SetRelativeScale3D (Variables|Default|GetTop) (Math|Vector|MakeVector _x_2 (Variables|Default|GetLenght) _z_2))
  (bind _returnvalue_16 (AddComponent|AddStaticMeshComponent false _returnvalue_9))
  (Rendering|Material|SetMaterial _returnvalue_16 0 (Variables|Default|GetElement%200))
  (Rendering|Material|SetMaterial _returnvalue_16 1 (Variables|Default|GetElement%201))
  (Rendering|Material|SetMaterial _returnvalue_16 2 (Variables|Default|GetElement%202))
  (bind _returnvalue_17 (AddComponent|AddStaticMeshComponent false _returnvalue_9))
  (Rendering|Material|SetMaterial _returnvalue_17 0 _element_0)
  (Rendering|Material|SetMaterial _returnvalue_17 1 (Variables|Default|GetElement%201))
  (Rendering|Material|SetMaterial _returnvalue_17 2 (Variables|Default|GetElement%202))
  (bind _returnvalue_18 (Rendering|Material|CreateDynamicMaterialInstance _returnvalue_17 0 _element_0 :!class /Script/Engine.PrimitiveComponent))
  (Rendering|Material|SetScalarParameterValue _returnvalue_18 "Tile_U" _returnvalue_2 :!class /Script/Engine.MaterialInstanceDynamic)
  (bind _returnvalue_19 (Rendering|Material|CreateDynamicMaterialInstance _returnvalue_17 2 (Variables|Default|GetElement%202) :!class /Script/Engine.PrimitiveComponent))
  (Rendering|Material|SetScalarParameterValue _returnvalue_19 "Tile_V" _returnvalue_2 :!class /Script/Engine.MaterialInstanceDynamic)
  (Transformation|SetRelativeScale3D _returnvalue_17 (Math|Vector|MakeVector (.X (Math|Vector|BreakVector (Variables|/Script/Engine.SceneComponent|GetRelativeScale3D _returnvalue_17))) (Variables|Default|GetLenght) (.Z (Math|Vector|BreakVector (Variables|/Script/Engine.SceneComponent|GetRelativeScale3D _returnvalue_17)))))
  (bind _returnvalue_20 (AddComponent|AddStaticMeshComponent false _returnvalue_4))
  (Rendering|Material|SetMaterial _returnvalue_20 0 _element_0_2)
  (Rendering|Material|SetMaterial _returnvalue_20 1 (Variables|Default|GetElement%201))
  (Rendering|Material|SetMaterial _returnvalue_20 2 (Variables|Default|GetElement%202))
  (bind _returnvalue_21 (Rendering|Material|CreateDynamicMaterialInstance _returnvalue_20 0 _element_0_2 :!class /Script/Engine.PrimitiveComponent))
  (Rendering|Material|SetScalarParameterValue _returnvalue_21 "Tile_U" _returnvalue_2 :!class /Script/Engine.MaterialInstanceDynamic)
  (bind _returnvalue_22 (Rendering|Material|CreateDynamicMaterialInstance _returnvalue_20 2 (Variables|Default|GetElement%202) :!class /Script/Engine.PrimitiveComponent))
  (Rendering|Material|SetScalarParameterValue _returnvalue_22 "Tile_V" _returnvalue_2 :!class /Script/Engine.MaterialInstanceDynamic)
  (Transformation|SetRelativeScale3D _returnvalue_20 (Math|Vector|MakeVector (.X (Math|Vector|BreakVector (Variables|/Script/Engine.SceneComponent|GetRelativeScale3D _returnvalue_20))) (Variables|Default|GetLenght) (.Z (Math|Vector|BreakVector (Variables|/Script/Engine.SceneComponent|GetRelativeScale3D _returnvalue_20)))))
  (bind _returnvalue_23 (AddComponent|AddStaticMeshComponent false _returnvalue_4))
  (Rendering|Material|SetMaterial _returnvalue_23 0 (Variables|Default|GetElement%200))
  (Rendering|Material|SetMaterial _returnvalue_23 1 (Variables|Default|GetElement%201))
  (Rendering|Material|SetMaterial _returnvalue_23 2 (Variables|Default|GetElement%202))
  (bind _returnvalue_24 (Rendering|Material|CreateDynamicMaterialInstance (Variables|Default|GetSide) 2 (Variables|Default|GetElement%202) :!class /Script/Engine.PrimitiveComponent))
  (Rendering|Material|SetScalarParameterValue _returnvalue_24 "Tile_U" _returnvalue_13 :!class /Script/Engine.MaterialInstanceDynamic)
  (bind _returnvalue_25 (Rendering|Material|CreateDynamicMaterialInstance (Variables|Default|GetTop) 0 (Variables|Default|GetElement%202) :!class /Script/Engine.PrimitiveComponent))
  (Rendering|Material|SetScalarParameterValue _returnvalue_25 "Tile_U" _returnvalue_13 :!class /Script/Engine.MaterialInstanceDynamic)
  (Rendering|Material|SetScalarParameterValue _returnvalue_25 "Tile_V" _returnvalue_2 :!class /Script/Engine.MaterialInstanceDynamic)
  (bind _returnvalue_26 (Rendering|Material|CreateDynamicMaterialInstance (Variables|Default|GetSide) 0 (Variables|Default|GetElement%200) :!class /Script/Engine.PrimitiveComponent))
  (Rendering|Material|SetScalarParameterValue _returnvalue_26 "Tile_U" _returnvalue_13 :!class /Script/Engine.MaterialInstanceDynamic))