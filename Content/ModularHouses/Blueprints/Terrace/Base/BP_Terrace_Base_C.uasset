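; Modular house terrace base Blueprint that builds a piece sized by Width and Lenght in its construction script.
; Side and Top spline meshes span from StartTransform to the Width-based end, while four static meshes are added in pairs at both ends.
; Lenght scales Top and one mesh per end along Y.
; Dynamic instances of Element0 and Element1 materials derive Tile_U and Tile_V from these dimensions, adjusting texture tiling to size.
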(fn ConstructionScript
  (bind _top (Variables|Default|GetTop))
  (bind _element_1 (Variables|Default|GetElement%201))
  (bind _lenght (Variables|Default|GetLenght))
  (bind _element_1_2 (Variables|Default|GetElement%201))
  (bind _width (Variables|Default|GetWidth))
  (bind _end (Variables|Default|GetEnd))
  (bind _width_2 (Variables|Default|GetWidth))
  (bind _end_transform (Variables|Default|GetEnd%20transform))
  (bind _start_transform (Variables|Default|GetStart%20transform))
  (bind _returnvalue (/ _lenght 0.8))
  (bind (_location _rotation _scale) (Math|Transform|BreakTransform _start_transform))
  (bind (_x _y _z) (Math|Vector|BreakVector _end))
  (bind _returnvalue_2 (- _width_2 1.2e+02))
  (bind (_location_2 _rotation_2 _scale_2) (Math|Transform|BreakTransform _end_transform))
  (bind _relativescale3d (Variables|/Script/Engine.SceneComponent|GetRelativeScale3D _top))
  (bind (_x_2 _y_2 _z_2) (Math|Vector|BreakVector _relativescale3d))
  (bind _returnvalue_3 (Math|Vector|MakeVector _width _y _z))
  (bind _returnvalue_4 (Math|Conversions|ToTransform(Vector) _location))
  (bind _returnvalue_5 (Math|Vector|GetForwardVector _rotation))
  (bind _returnvalue_6 (Math|Vector|GetForwardVector _rotation_2))
  (bind _returnvalue_7 (- _location _location_2))
  (bind _returnvalue_8 (* _returnvalue_2 0.00625))
  (bind _returnvalue_9 (Math|Conversions|ToTransform(Vector) _returnvalue_3))
  (bind _returnvalue_10 (Math|Vector|VectorLength _returnvalue_7))
  (bind _returnvalue_11 (* _returnvalue_5 _scale))
  (bind _returnvalue_12 (* _returnvalue_6 _scale_2))
  (bind _returnvalue_13 (+ _returnvalue_8 0.7))
  (bind _returnvalue_14 (* _returnvalue_11 _returnvalue_10))
  (bind _returnvalue_15 (* _returnvalue_12 _returnvalue_10))
  (Rendering|Material|SetMaterial (Variables|Default|GetTop) 0 (Variables|Default|GetElement%201))
  (SplineMesh|SetStartandEnd (Variables|Default|GetSide) _location _returnvalue_14 _returnvalue_3 _returnvalue_15 true :!class /Script/Engine.SplineMeshComponent)
  (SplineMesh|SetStartandEnd (Variables|Default|GetTop) _location _returnvalue_14 _returnvalue_3 _returnvalue_15 true :!class /Script/Engine.SplineMeshComponent)
  (Transformation|SetRelativeScale3D (Variables|Default|GetTop) (Math|Vector|MakeVector _x_2 (Variables|Default|GetLenght) _z_2))
  (bind _returnvalue_16 (AddComponent|AddStaticMeshComponent false _returnvalue_9))
  (Rendering|Material|SetMaterial _returnvalue_16 0 (Variables|Default|GetElement%200))
  (Rendering|Material|SetMaterial _returnvalue_16 1 (Variables|Default|GetElement%201))
  (bind _returnvalue_17 (AddComponent|AddStaticMeshComponent false _returnvalue_9))
  (Rendering|Material|SetMaterial _returnvalue_17 0 (Variables|Default|GetElement%200))
  (Rendering|Material|SetMaterial _returnvalue_17 1 _element_1)
  (bind _returnvalue_18 (Rendering|Material|CreateDynamicMaterialInstance _returnvalue_17 1 _element_1 :!class /Script/Engine.PrimitiveComponent))
  (Rendering|Material|SetScalarParameterValue _returnvalue_18 "Tile_V" _returnvalue :!class /Script/Engine.MaterialInstanceDynamic)
  (Transformation|SetRelativeScale3D _returnvalue_17 (Math|Vector|MakeVector (.X (Math|Vector|BreakVector (Variables|/Script/Engine.SceneComponent|GetRelativeScale3D _returnvalue_17))) (Variables|Default|GetLenght) (.Z (Math|Vector|BreakVector (Variables|/Script/Engine.SceneComponent|GetRelativeScale3D _returnvalue_17)))))
  (bind _returnvalue_19 (AddComponent|AddStaticMeshComponent false _returnvalue_4))
  (Rendering|Material|SetMaterial _returnvalue_19 0 (Variables|Default|GetElement%200))
  (Rendering|Material|SetMaterial _returnvalue_19 1 _element_1_2)
  (bind _returnvalue_20 (Rendering|Material|CreateDynamicMaterialInstance _returnvalue_19 1 _element_1_2 :!class /Script/Engine.PrimitiveComponent))
  (Rendering|Material|SetScalarParameterValue _returnvalue_20 "Tile_V" _returnvalue :!class /Script/Engine.MaterialInstanceDynamic)
  (Transformation|SetRelativeScale3D _returnvalue_19 (Math|Vector|MakeVector (.X (Math|Vector|BreakVector (Variables|/Script/Engine.SceneComponent|GetRelativeScale3D _returnvalue_19))) (Variables|Default|GetLenght) (.Z (Math|Vector|BreakVector (Variables|/Script/Engine.SceneComponent|GetRelativeScale3D _returnvalue_19)))))
  (bind _returnvalue_21 (AddComponent|AddStaticMeshComponent false _returnvalue_4))
  (Rendering|Material|SetMaterial _returnvalue_21 0 (Variables|Default|GetElement%200))
  (Rendering|Material|SetMaterial _returnvalue_21 1 (Variables|Default|GetElement%201))
  (bind _returnvalue_22 (Rendering|Material|CreateDynamicMaterialInstance (Variables|Default|GetSide) 1 (Variables|Default|GetElement%201) :!class /Script/Engine.PrimitiveComponent))
  (Rendering|Material|SetScalarParameterValue _returnvalue_22 "Tile_U" _returnvalue_13 :!class /Script/Engine.MaterialInstanceDynamic)
  (bind _returnvalue_23 (Rendering|Material|CreateDynamicMaterialInstance (Variables|Default|GetTop) 0 (Variables|Default|GetElement%201) :!class /Script/Engine.PrimitiveComponent))
  (Rendering|Material|SetScalarParameterValue _returnvalue_23 "Tile_U" _returnvalue_13 :!class /Script/Engine.MaterialInstanceDynamic)
  (Rendering|Material|SetScalarParameterValue _returnvalue_23 "Tile_V" (/ (Variables|Default|GetLenght) 0.8) :!class /Script/Engine.MaterialInstanceDynamic)
  (bind _returnvalue_24 (Rendering|Material|CreateDynamicMaterialInstance (Variables|Default|GetSide) 0 (Variables|Default|GetElement%200) :!class /Script/Engine.PrimitiveComponent))
  (Rendering|Material|SetScalarParameterValue _returnvalue_24 "Tile_U" _returnvalue_13 :!class /Script/Engine.MaterialInstanceDynamic))